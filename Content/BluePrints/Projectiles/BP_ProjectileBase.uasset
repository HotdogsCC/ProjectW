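; Base wizard projectile Blueprint that, on the server once ready, resolves overlaps into damage or explosions.
; Hits damage non-owner wizards, then spawn BP_ExplosionBase and destroy the projectile, as do other non-projectile overlaps.
; In projectile collisions, an explosive one detonates via BigBoomBoom, with the other projectile taking priority.
; BigBoomBoom draws a debug sphere, applies magic collision damage to wizards within the explosive radius, then destroys itself.
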(event Collision|EventActorBeginOverlap
  (params (OtherActor :type Actor%20Object%20Reference))
  ;[1 1 1] is this the server
  (if (Ability|HasAuthority)
    ;[1 1 1] are we ready to check for collisions
    (if (Class|ProjectileBase|GetReady)
      ;[1 1 1] is this a character?
      (bind _aswizard_character (Utilities|Casting|CastToWizardCharacter OtherActor)
        (:then
          ;[1 1 1] is this the character that spawned the projectile?
          (if (not (== (Class|ProjectileBase|GetWizardOwner) _aswizard_character))
            ;[1 1 1] deal damage to enemy
            (Class|WizardCharacter|TakeDamage _aswizard_character (Class|ProjectileBase|GetDamage))
            ;[1 1 1] spawn particles
            (Game|SpawnActorfromClass "/Game/BluePrints/Explosions/BP_ExplosionBase.BP_ExplosionBase_C" (Math|Transform|MakeTransform (Transformation|GetActorLocation) "0, 0, 0" "1.000000,1.000000,1.000000") "Undefined" "MultiplyWithRoot" 0 0 :!label _label)
            ;[1 1 1] destroy
            (Actor|DestroyActor)))
        (:CastFailed
          ;[1 1 1] is this another projectile?
          (bind _asprojectile_base (Utilities|Casting|CastToProjectileBase OtherActor)
            (:then
              ;[1 1 1] is the other projectile explosive?
              (if (Class|ProjectileBase|GetExplosive _asprojectile_base)
                ;[1 1 1] make it blow up
                (bind _asbp_projectile_base (Utilities|Casting|CastToBP_ProjectileBase _asprojectile_base))
                (CallFunction|BigBoomBoom _asbp_projectile_base)
                (goto _label)
                (else
                  ;[1 1 1] is this projectile explosive?
                  (if (Class|ProjectileBase|GetExplosive)
                    ;[1 1 1] blow us the fuck up
                    (CallFunction|BigBoomBoom)
                    (else
                      (goto _label))))))
            (:CastFailed
              (goto _label))))))))

(fn ConstructionScript)

(fn BigBoomBoom
  (bind _returnvalue (Transformation|GetActorLocation))
  (bind _returnvalue_2 (Class|ProjectileBase|GetExplosiveRadius))
  (Rendering|Debug|DrawDebugSphere _returnvalue _returnvalue_2 24 "(R=1.000000,G=1.000000,B=1.000000,A=1.000000)" 5.0)
  (bind _outactors (Collision|SphereOverlapActors _returnvalue _returnvalue_2 (Utilities|Array|MakeArray "ObjectTypeQuery3") 0))
  (for _array_element _outactors
    (bind _aswizard_character (Utilities|Casting|CastToWizardCharacter _array_element))
    (Class|WizardCharacter|TakeDamage _aswizard_character (Class|ProjectileBase|GetMagicCollisionDamage)))
  ;[1 1 1] destroy this projectile
  (Actor|DestroyActor))