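; JohnProjectile is a simple projectile actor that flies along its local X axis at a rate set by JohnSpeed.
; Tick scales the movement by delta time, then spins the Sphere component by a fixed step each frame, so the spin depends on frame rate.
; The sphere also jitters in size, taking a random uniform scale between one and two every frame.
; The graph contains no hit, damage or destroy logic.
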(event EventBeginPlay)

(event Collision|EventActorBeginOverlap
  (params (OtherActor :type Actor%20Object%20Reference)))

(event EventTick
  (params (DeltaSeconds :type Float%20%28single-precision%29))
  (bind _sphere (Variables|Default|GetSphere))
  (Transformation|AddActorLocalOffset (Math|Vector|MakeVector (* DeltaSeconds (Variables|Default|GetJohnSpeed)) 0.0 0.0) false false)
  (Transformation|AddRelativeRotation _sphere "0.000000,5.000000,0.000000" false false)
  (Transformation|SetRelativeScale3D _sphere (Math|Conversions|ToVector(Float) (+ (Math|Random|RandomFloat) 1.0))))

(fn ConstructionScript)